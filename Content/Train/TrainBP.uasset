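; TrainBP is a train actor that moves a Cube along its Spline in a continuous loop.
; On BeginPlay, a timeline's Anim value scales the spline length into a distance, and each update sets the cube's world location and rotation from that point at unit scale.
; When the timeline finishes it sets an AnimFinished flag, which Tick polls to clear and replay the timeline from the start.
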(event EventBeginPlay
  (bind _spline (Variables|Default|GetSpline))
  (bind _anim (Timeline|Timeline_0 PlayFromStart)
    (:Update
      (Transformation|SetWorldTransform (Variables|Default|GetCube) (Math|Transform|MakeTransform (Spline|GetLocationatDistanceAlongSpline _spline (* (Spline|GetSplineLength _spline) _anim) "World") (Spline|GetRotationatDistanceAlongSpline _spline (* (Spline|GetSplineLength _spline) _anim) "World")) false false))
    (:Finished
      (Variables|Default|SetanimFinished true))))

(event EventTick
  (params (DeltaSeconds :type Float%20%28single-precision%29))
  (bind _spline (Variables|Default|GetSpline))
  (if (Variables|Default|GetanimFinished)
    (Variables|Default|SetanimFinished false)
    (bind _anim (Timeline|Timeline_0 PlayFromStart)
      (:Update
        (Transformation|SetWorldTransform (Variables|Default|GetCube) (Math|Transform|MakeTransform (Spline|GetLocationatDistanceAlongSpline _spline (* (Spline|GetSplineLength _spline) _anim) "World") (Spline|GetRotationatDistanceAlongSpline _spline (* (Spline|GetSplineLength _spline) _anim) "World")) false false))
      (:Finished
        (Variables|Default|SetanimFinished true)))))

(fn ConstructionScript)