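; A one-shot trigger actor that plays a chain of level sequences when the toy car overlaps it, locking the car's movement during playback.
; The overlap starts the Lounge sequence, and each sequence's stop event re-binds to the same handler.
; That handler uses an incrementing counter to play TimerPuzzle, then FrictionPuzzle, and finally lets the car move again.
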(event Custom|OnStop_Event_0
  (bind _result (Math|Integer|IncrementInt (Variables|Default|GetCounter))
    (:%20%20
      (switch int _result
        (:0
          (bind _outactor (Sequencer|Player|CreateLevelSequencePlayer "/Game/LevelSequence/TimerPuzzle.TimerPuzzle"))
          (EventDispatchers|AssignOnStop (Variables|/Script/LevelSequence.LevelSequenceActor|GetSequencePlayer _outactor) (delegate Custom|OnStop_Event_0))
          (Sequencer|Player|Play (Variables|/Script/LevelSequence.LevelSequenceActor|GetSequencePlayer _outactor) :!class /Script/MovieScene.MovieSceneSequencePlayer))
        (:1
          (bind _outactor_2 (Sequencer|Player|CreateLevelSequencePlayer "/Game/LevelSequence/FrictionPuzzle.FrictionPuzzle"))
          (EventDispatchers|AssignOnStop (Variables|/Script/LevelSequence.LevelSequenceActor|GetSequencePlayer _outactor_2) (delegate Custom|OnStop_Event_0))
          (Sequencer|Player|Play (Variables|/Script/LevelSequence.LevelSequenceActor|GetSequencePlayer _outactor_2) :!class /Script/MovieScene.MovieSceneSequencePlayer))
        (:2
          (Class|ToyCar|SetCanMove (stale Collision|EventActorBeginOverlap _astoy_car) true))))))

(event Collision|EventActorBeginOverlap
  (params (OtherActor :type Actor%20Object%20Reference))
  (if (not (Variables|Default|GetHasBeenPlayed))
    (bind _astoy_car (Utilities|Casting|CastToToyCar OtherActor))
    (Class|ToyCar|SetCanMove _astoy_car false)
    (Variables|Default|SetHasBeenPlayed true)
    (bind _outactor (Sequencer|Player|CreateLevelSequencePlayer "/Game/LevelSequence/Lounge.Lounge"))
    (EventDispatchers|AssignOnStop (Variables|/Script/LevelSequence.LevelSequenceActor|GetSequencePlayer _outactor) (delegate Custom|OnStop_Event_0))
    (Sequencer|Player|Play (Variables|/Script/LevelSequence.LevelSequenceActor|GetSequencePlayer _outactor) :!class /Script/MovieScene.MovieSceneSequencePlayer)))

(fn ConstructionScript)