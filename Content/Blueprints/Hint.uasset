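; Hint trigger actor that shows a hint widget when the toy car overlaps it and can see hints.
; The hint's puzzle name selects a completion flag on the car, which ShowAfterPuzzleCompleted matches to show hints before or after completion.
; Hints without a puzzle show only once.
; A one-second Delay loop counts down, then removes the widget and resets the timer, ending early if the car's hint visibility turns off.
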(event Collision|EventActorBeginOverlap
  (params (OtherActor :type Actor%20Object%20Reference))
  (bind _showafterpuzzlecompleted (Variables|Default|GetShowAfterPuzzleCompleted))
  (if (not (Variables|Default|GetIsShowingHint))
    (bind _asmy_toy_car_bp (Utilities|Casting|CastToMyToyCarBP OtherActor))
    (if (Variables|/Script/GDP_Project.ToyCar|GetCanSeeHints _asmy_toy_car_bp)
      (switch Utilities|FlowControl|Switch|SwitchonPuzzleName (Variables|Default|GetPName)
        (:NewEnumerator0
          (if (Variables|/Script/GDP_Project.ToyCar|GetTimerPuzzleCompleted _asmy_toy_car_bp)
            (if _showafterpuzzlecompleted :!label _label
              (bind _returnvalue (UserInterface|CreateWidget (Variables|Default|GetHintWidget) (Game|GetPlayerController 0) :!label _label_2))
              (UserInterface|Viewport|AddtoViewport _returnvalue 0)
              (Variables|Default|SetIsShowingHint true)
              (Utilities|FlowControl|Delay 1.0 :!label _label_3)
              (if (Variables|/Script/GDP_Project.ToyCar|GetCanSeeHints _asmy_toy_car_bp)
                (if (>= (Variables|Default|GetRemaingTime) 0)
                  (Math|Integer|DecrementInt (Variables|Default|GetRemaingTime)
                    (:%20%20
                      (goto _label_3)))
                  (else
                    _)))
              (Widget|RemovefromParent _returnvalue)
              (Variables|Default|SetIsShowingHint false)
              (Variables|Default|SetRemaingTime 7))
            (else
              (if (not _showafterpuzzlecompleted) :!label _label_4
                (goto _label_2)))))
        (:NewEnumerator1
          (if (Variables|/Script/GDP_Project.ToyCar|GetFrictionPuzzleCompleted _asmy_toy_car_bp)
            (goto _label)
            (else
              (goto _label_4))))
        (:NewEnumerator2
          (if (Variables|/Script/GDP_Project.ToyCar|GetTrainPuzzleCompleted _asmy_toy_car_bp)
            (goto _label)
            (else
              (goto _label_4))))
        (:NewEnumerator4
          (if (not (Variables|Default|GetHasBeenSeen))
            (Variables|Default|SetHasBeenSeen true)
            (goto _label_2)))))))

(fn ConstructionScript)