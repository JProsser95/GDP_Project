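; Portal trigger Blueprint that lets the player's toy car teleport when it is not in a puzzle.
; On overlap it caches the car, sets CanTeleport from the car's puzzle state and shows an interact prompt, using a gamepad or standard widget to match the input.
; Ending overlap clears the flag and removes the prompt.
; HandleTeleport checks the flag, removes the widgets of all Hint actors, then calls Teleport.
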(event Collision|EventActorBeginOverlap
  (params (OtherActor :type Actor%20Object%20Reference))
  ;[1 1 1] When collided render the changer UI
  (bind _asmy_toy_car_bp (Utilities|Casting|CastToMyToyCarBP OtherActor))
  (bind _output_get (Variables|Default|SetpToyCar _asmy_toy_car_bp))
  (bind _returnvalue (Class|ToyCar|GetIsinPuzzle _output_get))
  (bind _output_get_2 (Variables|Default|SetCanTeleport (not _returnvalue)))
  (if _output_get_2
    ;;[1 1 1] Check if the user is playing with a gamepad
    (if (Variables|/Game/Blueprints/MyToyCarBP.MyToyCarBP_C|GetIsUsingGamePad _asmy_toy_car_bp)
      (bind _returnvalue_2 (UserInterface|CreateWidget "/Game/HUD/InteractWidgetController.InteractWidgetController_C"))
      (UserInterface|Viewport|AddtoViewport _returnvalue_2 0)
      (else
        (bind _returnvalue_3 (UserInterface|CreateWidget "/Game/HUD/InteractWidget.InteractWidget_C"))
        (UserInterface|Viewport|AddtoViewport _returnvalue_3 0)))))

(event Collision|EventActorEndOverlap
  (params (OtherActor :type Actor%20Object%20Reference))
  ;[1 1 1] If the player is no longer colliding with the trigger box, remove the UI
  (Variables|Default|SetCanTeleport false)
  (bind _asmy_toy_car_bp (Utilities|Casting|CastToMyToyCarBP OtherActor))
  (if (Variables|/Game/Blueprints/MyToyCarBP.MyToyCarBP_C|GetIsUsingGamePad _asmy_toy_car_bp)
    (Widget|RemovefromParent (stale Collision|EventActorBeginOverlap _returnvalue_2))
    (else
      (Widget|RemovefromParent (stale Collision|EventActorBeginOverlap _returnvalue_3)))))

(fn ConstructionScript)

(fn HandleTeleport
  (if (Variables|Default|GetCanTeleport)
    (bind _outactors (Actor|GetAllActorsOfClass "/Game/Blueprints/Hint.Hint_C"))
    (for _array_element _outactors
      (Default|RemoveWidget _array_element))
    (Class|Portal|Teleport)))