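; Player-controlled toy car Blueprint that handles pausing, HUD visibility, interaction and achievement triggers.
; Overlap events toggle an interact flag, letting keyboard or gamepad input cast the overlapped actor to use portals, switch possession or start timed puzzles.
; The car HUD appears on play, toggle or plane part pickup, then auto-hides after a short delay.
; Portal use with completed puzzles and a broken-vase counter award achievements through AchievementManagerBP.
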(event EventBeginPlay
  ;[1 1 1] Render the car HUD
  ;;[1 1 1] Cheack if a reference to the car HUD already exists
  (Utilities|IsValid (Variables|Default|GetCar%20HUD%20Reference)
    (:Is%20Valid
      _)
    (:Is%20Not%20Valid
      ;;[1 1 1] Create a reference to the car HUD
      (bind _returnvalue (UserInterface|CreateWidget "/Game/HUD/CarHUD.CarHUD_C"))
      (Variables|Default|SetCar%20HUD%20Reference _returnvalue)))
  ;;[1 1 1] Create the car HUD
  (UserInterface|Viewport|AddtoViewport (Variables|Default|GetCar%20HUD%20Reference) 0)
  (Utilities|FlowControl|Delay 3.0)
  (Widget|RemovefromParent (Variables|Default|GetCar%20HUD%20Reference))
  (Variables|Default|SetHideHUD true))

(event Collision|EventActorEndOverlap
  (params (OtherActor :type Actor%20Object%20Reference))
  (Variables|Default|SetCanInteract false))

(event EventUpdatePlanePartsinHUD
  (params (PlanePartNumber :type Integer))
  ;[1 1 1] Update the Car HUD with the plane part that has just been picked up by the player
  (Default|UpdatePlaneParts (Variables|Default|GetCar%20HUD%20Reference) PlanePartNumber)
  (Variables|Default|SetHideHUD false)
  ;[1 1 1] Render the car HUD
  ;;[1 1 1] Create the car HUD
  (UserInterface|Viewport|AddtoViewport (Variables|Default|GetCar%20HUD%20Reference) 0)
  (Utilities|FlowControl|Delay 3.0)
  (Widget|RemovefromParent (Variables|Default|GetCar%20HUD%20Reference))
  (Variables|Default|SetHideHUD true))

(event Collision|EventActorBeginOverlap
  (params (OtherActor :type Actor%20Object%20Reference))
  (Variables|Default|SetCanInteract true))

(event Input|GamepadEvents|GamepadSpecialRight
  (params (Key :type Key%20Structure))
  (bind _returnvalue (Game|GetPlayerController 0))
  ;[1 1 1] Pause the Game
  (:Released
    (if (not (Variables|Default|GetGameIsLoading))
      ;;[1 1 1] Check if a reference to the pause menu already exists
      (Utilities|IsValid (Variables|Default|GetPause%20Menu%20Reference)
        (:Is%20Valid
          _)
        (:Is%20Not%20Valid
          ;;[1 1 1] Create a reference to the pause menu
          (bind _returnvalue_2 (UserInterface|CreateWidget "/Game/Menus/PauseMenu.PauseMenu_C"))
          (Variables|Default|SetPause%20Menu%20Reference _returnvalue_2)))
      ;;[1 1 1] Create the pause menu
      (Input|SetInputModeUIOnly _returnvalue (Variables|Default|GetPause%20Menu%20Reference) "DoNotLock")
      (UserInterface|Viewport|AddtoViewport (Variables|Default|GetPause%20Menu%20Reference) 0)
      (Widget|SetKeyboardFocus (Variables|Default|GetPause%20Menu%20Reference))
      (Variables|/Script/Engine.PlayerController|SetbShowMouseCursor _returnvalue true)
      (Game|SetGamePaused true))))

(event Input|KeyboardEvents|P
  (params (Key :type Key%20Structure))
  (bind _returnvalue (Game|GetPlayerController 0))
  ;[1 1 1] Pause the Game
  (:Released
    (if (not (Variables|Default|GetGameIsLoading))
      ;;[1 1 1] Check if a reference to the pause menu already exists
      (Utilities|IsValid (Variables|Default|GetPause%20Menu%20Reference)
        (:Is%20Valid
          _)
        (:Is%20Not%20Valid
          ;;[1 1 1] Create a reference to the pause menu
          (bind _returnvalue_2 (UserInterface|CreateWidget "/Game/Menus/PauseMenu.PauseMenu_C"))
          (Variables|Default|SetPause%20Menu%20Reference _returnvalue_2)))
      ;;[1 1 1] Create the pause menu
      (Input|SetInputModeUIOnly _returnvalue (Variables|Default|GetPause%20Menu%20Reference) "DoNotLock")
      (UserInterface|Viewport|AddtoViewport (Variables|Default|GetPause%20Menu%20Reference) 0)
      (Widget|SetKeyboardFocus (Variables|Default|GetPause%20Menu%20Reference))
      (Variables|/Script/Engine.PlayerController|SetbShowMouseCursor _returnvalue true)
      (Game|SetGamePaused true))))

(event Input|KeyboardEvents|AnyKey
  (params (Key :type Key%20Structure))
  ;[1 1 1] Find if the user is playing with a gamepad
  (:Pressed
    (Variables|Default|SetIsUsingGamePad (Class|KismetInputLibrary|KeyIsGamepadKey Key))))

(event Input|KeyboardEvents|H
  (params (Key :type Key%20Structure))
  ;[1 1 1] Hide the car HUD
  (:Pressed
    (bind _output_get (Variables|Default|SetHideHUD (not (Variables|Default|GetHideHUD))))
    (if _output_get
      (Widget|RemovefromParent (Variables|Default|GetCar%20HUD%20Reference))
      (else
        ;[1 1 1] Render the car HUD
        ;;[1 1 1] Cheack if a reference to the car HUD already exists
        (Utilities|IsValid (Variables|Default|GetCar%20HUD%20Reference)
          (:Is%20Valid
            _)
          (:Is%20Not%20Valid
            ;;[1 1 1] Create a reference to the car HUD
            (bind _returnvalue (UserInterface|CreateWidget "/Game/HUD/CarHUD.CarHUD_C"))
            (Variables|Default|SetCar%20HUD%20Reference _returnvalue)))
        ;;[1 1 1] Create the car HUD
        (UserInterface|Viewport|AddtoViewport (Variables|Default|GetCar%20HUD%20Reference) 0)
        (Utilities|FlowControl|Delay 3.0)
        (Widget|RemovefromParent (Variables|Default|GetCar%20HUD%20Reference))
        (Variables|Default|SetHideHUD true)))))

(event Input|KeyboardEvents|E
  (params (Key :type Key%20Structure))
  (:Released
    (if (Variables|Default|GetCanInteract)
      (bind _asmy_portal_bp (Utilities|Casting|CastToMyPortalBP (stale Collision|EventActorBeginOverlap OtherActor))
        (:then
          (Default|HandleTeleport _asmy_portal_bp)
          (if (and (Variables|Default|GetTimerPuzzleCompleted) (Variables|Default|GetFrictionPuzzleCompleted))
            (bind _outactors (Actor|GetAllActorsOfClass "/Game/Blueprints/AchievementManagerBP.AchievementManagerBP_C"))
            (Class|AchievementManager|EarnAchievement _outactors "LOUNGE_COMPLETE"))
          (if (Variables|Default|GetTrainPuzzleCompleted)
            (bind _outactors_2 (Actor|GetAllActorsOfClass "/Game/Blueprints/AchievementManagerBP.AchievementManagerBP_C"))
            (Class|AchievementManager|EarnAchievement _outactors_2 "PLAYROOM_COMPLETE")))
        (:CastFailed
          (bind _asmy_possession_changer_bp (Utilities|Casting|CastToMyPossessionChangerBP (stale Collision|EventActorBeginOverlap OtherActor))
            (:then
              (Variables|/Game/Blueprints/MyPossessionChangerBP.MyPossessionChangerBP_C|SetPossessionCalled _asmy_possession_changer_bp true)
              (Default|ChangePossession _asmy_possession_changer_bp self))
            (:CastFailed
              (bind _astime_puzzle_bp (Utilities|Casting|CastToTimePuzzleBP (stale Collision|EventActorBeginOverlap OtherActor)))
              (Variables|/Game/Blueprints/TimePuzzleBP.TimePuzzleBP_C|SetPuzzleBeginPressed _astime_puzzle_bp true))))))))

(event Input|GamepadEvents|GamepadFaceButtonTop
  (params (Key :type Key%20Structure))
  (:Released
    (if (Variables|Default|GetCanInteract)
      (bind _asmy_portal_bp (Utilities|Casting|CastToMyPortalBP (stale Collision|EventActorBeginOverlap OtherActor))
        (:then
          (Default|HandleTeleport _asmy_portal_bp)
          (if (and (Variables|Default|GetTimerPuzzleCompleted) (Variables|Default|GetFrictionPuzzleCompleted))
            (bind _outactors (Actor|GetAllActorsOfClass "/Game/Blueprints/AchievementManagerBP.AchievementManagerBP_C"))
            (Class|AchievementManager|EarnAchievement _outactors "LOUNGE_COMPLETE"))
          (if (Variables|Default|GetTrainPuzzleCompleted)
            (bind _outactors_2 (Actor|GetAllActorsOfClass "/Game/Blueprints/AchievementManagerBP.AchievementManagerBP_C"))
            (Class|AchievementManager|EarnAchievement _outactors_2 "PLAYROOM_COMPLETE")))
        (:CastFailed
          (bind _asmy_possession_changer_bp (Utilities|Casting|CastToMyPossessionChangerBP (stale Collision|EventActorBeginOverlap OtherActor))
            (:then
              (Variables|/Game/Blueprints/MyPossessionChangerBP.MyPossessionChangerBP_C|SetPossessionCalled _asmy_possession_changer_bp true)
              (Default|ChangePossession _asmy_possession_changer_bp self))
            (:CastFailed
              (bind _astime_puzzle_bp (Utilities|Casting|CastToTimePuzzleBP (stale Collision|EventActorBeginOverlap OtherActor)))
              (Variables|/Game/Blueprints/TimePuzzleBP.TimePuzzleBP_C|SetPuzzleBeginPressed _astime_puzzle_bp true))))))))

(fn ConstructionScript)

(fn BreakVase
  (bind _result (Math|Integer|IncrementInt (Variables|Default|GetVasesBroken))
    (:%20%20
      (if (== _result 4)
        (bind _outactors (Actor|GetAllActorsOfClass "/Game/Blueprints/AchievementManagerBP.AchievementManagerBP_C"))
        (Class|AchievementManager|EarnAchievement _outactors "SMASH_ALL_VASES")))))