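; Trigger actor that shows an interact prompt for changing possession while a MyToyCarBP overlaps it.
; Begin overlap creates either a controller or keyboard prompt widget based on the car's IsUsingGamePad flag, and end overlap removes it.
; Both overlap events do nothing once PossessionCalled is true.
; ChangePossession only removes the stored prompt widget; this Blueprint neither sets that flag nor possesses anything.
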(event Collision|EventActorBeginOverlap
  (params (OtherActor :type Actor%20Object%20Reference))
  ;[1 1 1] When collided render the changer UI
  (if (not (Variables|Default|GetPossessionCalled))
    ;;[1 1 1] Check if the user is playing with a gamepad
    (bind _asmy_toy_car_bp (Utilities|Casting|CastToMyToyCarBP OtherActor))
    (if (Variables|/Game/Blueprints/MyToyCarBP.MyToyCarBP_C|GetIsUsingGamePad _asmy_toy_car_bp)
      (bind _returnvalue (UserInterface|CreateWidget "/Game/HUD/InteractWidgetController.InteractWidgetController_C"))
      (UserInterface|Viewport|AddtoViewport _returnvalue 0)
      (Variables|Default|SetControllerWidget _returnvalue)
      (else
        (bind _returnvalue_2 (UserInterface|CreateWidget "/Game/HUD/InteractWidget.InteractWidget_C"))
        (UserInterface|Viewport|AddtoViewport _returnvalue_2 0)
        (Variables|Default|SetKeyboardWidget _returnvalue_2)))))

(event Collision|EventActorEndOverlap
  (params (OtherActor :type Actor%20Object%20Reference))
  ;[1 1 1] If the player is no longer colliding with the trigger box, remove the UI
  (if (not (Variables|Default|GetPossessionCalled))
    (bind _asmy_toy_car_bp (Utilities|Casting|CastToMyToyCarBP OtherActor))
    (if (Variables|/Game/Blueprints/MyToyCarBP.MyToyCarBP_C|GetIsUsingGamePad _asmy_toy_car_bp)
      (Widget|RemovefromParent (stale Collision|EventActorBeginOverlap _returnvalue))
      (else
        (Widget|RemovefromParent (stale Collision|EventActorBeginOverlap _returnvalue_2))))))

(fn ConstructionScript)

(fn ChangePossession
  (params (other%20actor :type Actor%20Object%20Reference))
  (bind _asmy_toy_car_bp (Utilities|Casting|CastToMyToyCarBP other%20actor))
  (if (Variables|/Game/Blueprints/MyToyCarBP.MyToyCarBP_C|GetIsUsingGamePad _asmy_toy_car_bp)
    (Widget|RemovefromParent (Variables|Default|GetControllerWidget))
    (else
      (Widget|RemovefromParent (Variables|Default|GetKeyboardWidget)))))