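; Breakable vase actor that shatters on impact and can award an achievement.
; On a hit, it applies damage to its VaseDM destructible mesh at the impact point along the impulse, then switches that mesh to physics-only collision.
; If the hit actor's first tag is "Ball", it finds AchievementManagerBP in the level and earns the WING achievement.
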(event EventBeginPlay)

(event Collision|EventActorBeginOverlap
  (params (OtherActor :type Actor%20Object%20Reference)))

(event EventTick
  (params (DeltaSeconds :type Float%20%28single-precision%29)))

(event Collision|EventHit
  (params (MyComp :type Primitive%20Component%20Object%20Reference) (Other :type Actor%20Object%20Reference) (OtherComp :type Primitive%20Component%20Object%20Reference) (bSelfMoved :type Boolean) (HitLocation :type Vector :default "0, 0, 0") (HitNormal :type Vector :default "0, 0, 0") (NormalImpulse :type Vector :default "0, 0, 0") (Hit :type Hit%20Result%20Structure%20%28by%20ref%29))
  (Class|DestructibleComponent|ApplyDamage (Variables|Default|GetVase_DM) 1.0 HitLocation NormalImpulse 0.0)
  (Collision|SetCollisionEnabled (Variables|Default|GetVase_DM) "PhysicsOnly")
  (if (Utilities|Enum|Equal(Enum) (Utilities|String|ToString(Name) (Utilities|Array|Get(acopy) (Variables|/Script/Engine.Actor|GetTags (.HitActor (Collision|BreakHitResult Hit))))) "Ball")
    (bind _outactors (Actor|GetAllActorsOfClass "/Game/Blueprints/AchievementManagerBP.AchievementManagerBP_C"))
    (Class|AchievementManager|EarnAchievement _outactors "PLANE_WING")))

(fn ConstructionScript)